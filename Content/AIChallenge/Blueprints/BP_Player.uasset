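; Player Blueprint for the AI Challenge that lets the user spawn NPCs by pointing with the mouse.
; On BeginPlay it shows the mouse cursor.
; The SpawnNPC input deprojects the cursor into the world and line traces on the Visibility channel up to TraceDistance.
; If the trace hits a BP_SpawnArea, it spawns a PolygonCharacterNPC_BP at the hit location.
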(event `self.ReceiveBeginPlay`
  (set `PlayerController.bShowMouseCursor` true (`GameplayStatics.GetPlayerController` 0)))

(event `InputAction|SpawnNPC`
  (params (Key :type "Key Structure"))
  (bind (_worldlocation _worlddirection) (`PlayerController.DeprojectMousePositionToWorld` (`GameplayStatics.GetPlayerController` 0)))
  (:`Pressed`
    (bind _outhit (`KismetSystemLibrary.LineTraceSingle` _worldlocation (+ _worldlocation (* _worlddirection (`self.TraceDistance`))) "TraceTypeQuery1"))
    (bind (_bblockinghit _binitialoverlap _time _distance _location _impactpoint _normal _impactnormal _physmat _hitactor) (`GameplayStatics.BreakHitResult` _outhit))
    (cast `/Game/AIChallenge/Blueprints/BP_SpawnArea` _hitactor)
    (`|SpawnActorFromClass` "/Game/AIChallenge/Blueprints/PolygonCharacterNPC_BP.PolygonCharacterNPC_BP_C" (`KismetMathLibrary.MakeTransform` _location) "Undefined" "OverrideRootScale" null null)))

(fn `UserConstructionScript`)